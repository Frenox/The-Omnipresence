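; BP_C_Character is a character that patrols a list of target actors when tagged "Patrol".
; After a short delay on BeginPlay, it uses AI MoveTo toward the first valid target.
; On success it rotates that target to the back of the list, waits, then repeats, forming an endless loop.
; A randomized Move event exists, but its only call here is disconnected.
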(event Custom|Move
  (Class|CCharacter|StartMove (Variables|Default|GetMvmt))
  (Utilities|FlowControl|Delay 0.2)
  (Variables|Default|SetMvmt (Math|Random|RandomInteger 3)))

(event Custom|Patrol
  (bind _targetlist (Variables|Default|GetTargetList))
  ;[1 1 1] Go to the exact location of an actor
  (bind _output_get (Variables|Default|SetTarget (Utilities|Array|Get(acopy) (Variables|Default|GetTargetList))))
  (Utilities|IsValid _output_get
    (:Is%20Valid
      (AI|AIMoveTo self "0, 0, 0" (Variables|Default|GetTarget) 1e+01 false
        (:OnSuccess
          (Utilities|Array|RemoveItem _targetlist (Variables|Default|GetTarget))
          (Utilities|Array|Add _targetlist (Variables|Default|GetTarget))
          (Utilities|FlowControl|Delay 4.0)
          (CallFunction|Patrol))))))

(event EventBeginPlay
  (if (Actor|ActorHasTag "Patrol")
    (Utilities|FlowControl|Delay 5.0)
    (CallFunction|Patrol)))

(event Collision|EventActorBeginOverlap
  (params (OtherActor :type Actor%20Object%20Reference)))

(event EventTick
  (params (DeltaSeconds :type Float%20%28single-precision%29)))

(fn ConstructionScript)