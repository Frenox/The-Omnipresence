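; AI character Blueprint that supplies patrol targets to its BP_CharacterController from a list of actors.
; SetPatrolLoc passes the first valid target to the controller's SetPatrol, then rotates it to the list's end for cyclic patrolling.
; UpdateWalkSpeed sets the movement component's max walk speed.
; Patrol is an empty event, and an older AIMoveTo patrol loop remains disconnected.
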(event Custom|Patrol
  ;[1 1 1] Go to the exact location of an actor
)

(event Custom|SetPatrolLoc
  (bind _targetlist (Variables|Default|GetTargetList))
  ;[1 1 1] Set Patrol location for AI
  (bind _output_get (Variables|Default|SetAIController (Pawn|GetController)))
  (bind _asbp_character_controller (Utilities|Casting|CastToBP_CharacterController _output_get))
  (bind _output_get_2 (Variables|Default|SetTarget (Utilities|Array|Get(acopy) (Variables|Default|GetTargetList))))
  (Utilities|IsValid _output_get_2
    (:Is%20Valid
      (Default|SetPatrol _asbp_character_controller _output_get_2)
      (Utilities|Array|RemoveItem _targetlist (Variables|Default|GetTarget))
      (Utilities|Array|Add _targetlist (Variables|Default|GetTarget)))))

(event EventBeginPlay)

(event Collision|EventActorBeginOverlap
  (params (OtherActor :type Actor%20Object%20Reference)))

(event EventTick
  (params (DeltaSeconds :type Float%20%28single-precision%29)))

(fn ConstructionScript)

(fn UpdateWalkSpeed
  (params (NewWalkSpeed :type Float%20%28single-precision%29))
  (Variables|/Script/Engine.CharacterMovementComponent|SetMaxWalkSpeed (Variables|Character|GetCharacterMovement) NewWalkSpeed))