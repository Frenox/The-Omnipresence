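; BP_MissionsManager tracks mission progression, showing and completing missions in on-screen BP_Mission widgets.
; MissionTrigger maps an actor to a DATA_Missions row and shows that mission once, if its PreviousMission is completed or "None".
; UpdateMission applies the same prerequisite, completes the matching widget or creates one, and records completion in MissionsStates.
; BeginPlay separately gathers display names of MissionTrigger-tagged actors into Actors.
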(event EventBeginPlay
  (bind _outactors (Actor|GetAllActorswithTag "MissionTrigger"))
  (for _array_element _outactors
    (Utilities|Array|AddUnique (Variables|Default|GetActors) (Utilities|GetDisplayName _array_element))))

(event Collision|EventActorBeginOverlap
  (params (OtherActor :type Actor%20Object%20Reference)))

(event EventTick
  (params (DeltaSeconds :type Float%20%28single-precision%29)))

(fn ConstructionScript)

(fn MissionTrigger
  (params (Actor :type String))
  (bind _missions (Variables|Default|GetMissions))
  (bind _value (Utilities|Map|Find _missions Actor))
  (bind _returnvalue (Utilities|GetDataTableRow "/Game/Missions/DATA_Missions.DATA_Missions" (Utilities|String|StringToName _value))
    (:then
      (if (not (.Value (Utilities|Map|Find (Variables|Default|GetMissionsTriggerStates) _value)))
        (if (or (.Value (Utilities|Map|Find (Variables|Default|GetMissionsStates) (.PreviousMission (Utilities|Struct|BreakSTRUCT_Missions _returnvalue)))) (Utilities|Enum|Equal(Enum) (.PreviousMission (Utilities|Struct|BreakSTRUCT_Missions _returnvalue)) "None"))
          (Utilities|Map|Add (Variables|Default|GetMissionsTriggerStates) _value true)
          (bind _returnvalue_2 (UserInterface|CreateWidget "/Game/Widgets/Missions/BP_Mission.BP_Mission_C"))
          (UserInterface|Viewport|AddtoViewport _returnvalue_2 0)
          (Default|ShowNewMission _returnvalue_2 (.Text (Utilities|Struct|BreakSTRUCT_Missions _returnvalue))))))))

(fn UpdateMission
  (params (Mission :type String))
  (bind _returnvalue (Utilities|GetDataTableRow "/Game/Missions/DATA_Missions.DATA_Missions" (Utilities|String|StringToName Mission))
    (:then
      (if (or (.Value (Utilities|Map|Find (Variables|Default|GetMissionsStates) (.PreviousMission (Utilities|Struct|BreakSTRUCT_Missions _returnvalue)))) (Utilities|Enum|Equal(Enum) (.PreviousMission (Utilities|Struct|BreakSTRUCT_Missions _returnvalue)) "None"))
        (bind _foundwidgets (Widget|GetAllWidgetsOfClass "/Game/Widgets/Missions/BP_Mission.BP_Mission_C" true))
        (bind _array_element (Utilities|Array|ForEachLoopwithBreak _foundwidgets)
          (:LoopBody
            (if (Utilities|Enum|Equal(Enum) (Variables|/Game/Widgets/Missions/BP_Mission.BP_Mission_C|GetCurrentMission _array_element) (.Text (Utilities|Struct|BreakSTRUCT_Missions _returnvalue)))
              (Default|MissionCompleted _array_element)
              (Utilities|Map|Add (Variables|Default|GetMissionsStates) Mission true :!label _label)
              (return)))
          (:Completed
            (bind _returnvalue_2 (UserInterface|CreateWidget "/Game/Widgets/Missions/BP_Mission.BP_Mission_C"))
            (UserInterface|Viewport|AddtoViewport _returnvalue_2 0)
            (Default|ShowNewMission _returnvalue_2 (.Text (Utilities|Struct|BreakSTRUCT_Missions _returnvalue)))
            (Default|MissionCompleted _returnvalue_2)
            (goto _label)))))))