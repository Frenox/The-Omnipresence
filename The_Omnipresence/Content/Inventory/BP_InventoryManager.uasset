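; Inventory manager actor that opens and closes the inventory UI and keeps basic inventory state.
; InventoryToggle creates or removes the BP_Inventory widget, toggles the mouse cursor, and passes the open state to BP_C_Player's SetMovementMode.
; ItemPicked only increments and prints an item count, ignoring the item name, while ChangeTab stores and prints the current tab.
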(event EventBeginPlay
  (Variables|Default|SetPlayer (Game|GetPlayerCharacter 0)))

(event Collision|EventActorBeginOverlap
  (params (OtherActor :type Actor%20Object%20Reference)))

(event EventTick
  (params (DeltaSeconds :type Float%20%28single-precision%29)))

(fn ConstructionScript)

(fn ItemPicked
  (params (Item_name :type String))
  (bind _output_get (Variables|Default|SetItemsAmount (+ (Variables|Default|GetItemsAmount) 1)))
  (Development|PrintString (Utilities|String|ToString(Integer) _output_get)))

(fn InventoryToggle
  (bind _returnvalue (Game|GetPlayerController 0))
  (if (Variables|Default|GetisOpen)
    (bind _foundwidgets (Widget|GetAllWidgetsOfClass "/Game/Widgets/Inventory/BP_Inventory.BP_Inventory_C" true))
    (Widget|RemovefromParent _foundwidgets)
    (Variables|Default|SetisOpen false)
    (Variables|/Script/Engine.PlayerController|SetbShowMouseCursor _returnvalue false)
    (else
      (bind _returnvalue_2 (UserInterface|CreateWidget "/Game/Widgets/Inventory/BP_Inventory.BP_Inventory_C"))
      (UserInterface|Viewport|AddtoViewport _returnvalue_2 0)
      (Variables|Default|SetisOpen true)
      (Variables|/Script/Engine.PlayerController|SetbShowMouseCursor _returnvalue true)))
  (bind _asbp_c_player (Utilities|Casting|CastToBP_C_Player (Variables|Default|GetPlayer)))
  (Default|SetMovementMode _asbp_c_player (Variables|Default|GetisOpen)))

(fn ChangeTab
  (params (Tab :type String))
  (bind _output_get (Variables|Default|SetcurrentTab Tab))
  (Development|PrintString _output_get))