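; Collectible item Blueprint that advances missions when an actor is interacted with.
; BeginPlay caches the player, game instance and an unused missions manager reference.
; Interact skips items already in the player's ItemsCollected map, otherwise updates or triggers missions by actor tag, increments the item count and records the item.
; FindPreviousMission reads the prior mission from DATA_Missions and calls UpdateMission itself, so updater items call it twice.
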(event EventBeginPlay
  (bind _asc_player (Utilities|Casting|CastToC_Player (Game|Player|GetPlayerPawn 0)))
  (Variables|Default|SetPlayer _asc_player)
  (bind _returnvalue (Actor|GetActorOfClass "/Game/Missions/BP_MissionsManager.BP_MissionsManager_C"))
  (Variables|Default|SetMissionsManagerRef _returnvalue)
  (bind _asbp_game_instance (Utilities|Casting|CastToBP_GameInstance (Game|GetGameInstance)))
  (Variables|Default|SetGameInstance _asbp_game_instance))

(event Collision|EventActorBeginOverlap
  (params (OtherActor :type Actor%20Object%20Reference)))

(event EventTick
  (params (DeltaSeconds :type Float%20%28single-precision%29)))

(event EventInteract
  (params (Actor :type String))
  (bind _gameinstance (Variables|Default|GetGameInstance))
  (if (not (.Value (Utilities|Map|Find (Variables|/Script/The_Omnipresence.C_Player|GetitemsCollected (Variables|Default|GetPlayer)) Actor)))
    (if (Actor|ActorHasTag "MissionUpdater")
      (bind _value (CallFunction|FindPreviousMission Actor))
      (Default|UpdateMission _gameinstance _value))
    (if (Actor|ActorHasTag "MissionTrigger")
      (Default|MissionTrigger _gameinstance Actor))
    (Default|IncrementItemsAmount (Variables|Default|GetGameInstance))
    (Utilities|Map|Add (Variables|/Script/The_Omnipresence.C_Player|GetitemsCollected (Variables|Default|GetPlayer)) Actor true)))

(fn ConstructionScript)

(fn FindPreviousMission
  (params (ItemToFind :type String%20%28by%20ref%29))
  (bind _returnvalue (Utilities|GetDataTableRow "/Game/Missions/DATA_Missions.DATA_Missions" (Utilities|String|StringToName (.Value (Utilities|Map|Find (Variables|/Game/BP_GameInstance.BP_GameInstance_C|GetMissions (Variables|Default|GetGameInstance)) ItemToFind))))
    (:then
      (Default|UpdateMission (Variables|Default|GetGameInstance) (.PreviousMission (Utilities|Struct|BreakSTRUCT_Missions _returnvalue)))
      (return (.PreviousMission (Utilities|Struct|BreakSTRUCT_Missions _returnvalue))))))