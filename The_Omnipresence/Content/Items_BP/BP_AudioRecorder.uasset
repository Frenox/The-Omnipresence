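; BP_AudioRecorder is an interactable audio recorder item that can be collected and can drive mission progress.
; On Interact, MissionUpdater and MissionTrigger tags decide whether it updates or triggers a mission through BP_MissionsManager.
; For updates, FindPreviousMission takes the Missions map entry one key before the item, relying on key order.
; It then notifies BP_InventoryManager of the pickup and flags "AudioRecorder" in the player's ItemsCollected map.
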(event EventBeginPlay)

(event Collision|EventActorBeginOverlap
  (params (OtherActor :type Actor%20Object%20Reference)))

(event EventTick
  (params (DeltaSeconds :type Float%20%28single-precision%29)))

(event EventInteract
  (params (Actor :type String))
  (bind _returnvalue (Actor|GetActorOfClass "/Game/Missions/BP_MissionsManager.BP_MissionsManager_C"))
  (if (Actor|ActorHasTag "MissionUpdater")
    (bind _value (CallFunction|FindPreviousMission _returnvalue Actor))
    (Default|UpdateMission _returnvalue _value))
  (if (Actor|ActorHasTag "MissionTrigger")
    (Default|MissionTrigger _returnvalue Actor))
  (bind _returnvalue_2 (Actor|GetActorOfClass "/Game/Inventory/BP_InventoryManager.BP_InventoryManager_C"))
  (Default|ItemPicked _returnvalue_2 Actor)
  (bind _asc_player (Utilities|Casting|CastToC_Player (Game|Player|GetPlayerPawn 0)))
  (Utilities|Map|Add (Variables|/Script/The_Omnipresence.C_Player|GetitemsCollected _asc_player) "AudioRecorder" true))

(fn ConstructionScript)

(fn FindPreviousMission
  (params (self2 :type BP%20Missions%20Manager%20Object%20Reference) (ItemToFind :type String%20%28by%20ref%29))
  (bind _missions (Variables|/Game/Missions/BP_MissionsManager.BP_MissionsManager_C|GetMissions self2))
  (bind _keys (Utilities|Map|Keys _missions))
  (return (.Value (Utilities|Map|Find _missions (Utilities|Array|Get(acopy) _keys (- (Utilities|Array|FindItem _keys ItemToFind) 1))))))