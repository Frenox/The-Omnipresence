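; BP_LevelChangerTrigger is a trigger actor that sends the player to another level.
; On BeginPlay it caches the player pawn as BP_C_Player.
; When that player begins overlapping it while IsActive is true, it calls ChangeLevel with a spawn point and the target level name prefixed with "LVL_".
; A SetTriggerActive event sets IsActive to true, so the trigger can be enabled externally.
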(event EventBeginPlay
  (bind _asbp_c_player (Utilities|Casting|CastToBP_C_Player (Game|GetPlayerCharacter 0)))
  (Variables|Default|SetPlayer _asbp_c_player))

(event Collision|EventActorBeginOverlap
  (params (OtherActor :type Actor%20Object%20Reference))
  (if (and (== OtherActor (Variables|Default|GetPlayer)) (Variables|Default|GetisActive))
    (CallFunction|ChangeLevel (Utilities|String|Append "LVL_" (Variables|Default|GetLevelToOpen)) (Variables|Default|GetSpawnPoint))))

(event EventTick
  (params (DeltaSeconds :type Float%20%28single-precision%29)))

(event EventSetTriggerActive
  (Variables|Default|SetisActive true))

(fn ConstructionScript)