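; House door actor that swings open or closed on Interact, ignoring requests while it is moving.
; Open and close loop one-degree yaw steps through short Delays, then snap to 130 degrees or the starting rotation.
; A child-actor NavLinkProxy's smart-link event lets BP_C_Character open a closed door, halting its movement for one second before restoring walking.
; The overlap-based opening logic is disconnected.
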(event Custom|CloseDoor
  ;[1 1 1] Close
  (Variables|Default|SetDoorTick 0)
  (if (< (Variables|Default|GetDoorTick) 131) :!label _label
    (Transformation|AddActorLocalRotation "0,-1.000000, 0" false false)
    (Math|Integer|IncrementInt (Variables|Default|GetDoorTick)
      (:%20%20
        (Utilities|FlowControl|Delay 0.001)
        (goto _label)))
    (else
      (Transformation|SetActorRelativeRotation (Variables|Default|GetOriginalRotation))
      (Variables|Default|SetIsOpen false)
      (Variables|Default|SetIsOpenning false))))

(event Custom|Link%20Reachedd
  (params (MovingActor :type Actor%20Object%20Reference) (DestinationPoint :type Vector%20%28by%20ref%29))
  (if (not (Variables|Default|GetIsOpen))
    (bind _asbp_c_character (Utilities|Casting|CastToBP_C_Character MovingActor))
    (Pawn|Components|CharacterMovement|SetMovementMode (Variables|/Script/Engine.Character|GetCharacterMovement _asbp_c_character) "MOVE_None" 0)
    (CallFunction|Interact)
    (Utilities|FlowControl|Delay 1.0)
    (Pawn|Components|CharacterMovement|SetMovementMode (Variables|/Script/Engine.Character|GetCharacterMovement _asbp_c_character) "MOVE_Walking" 0)))

(event Custom|OpenDoor
  (bind _originalrotation (Variables|Default|GetOriginalRotation))
  (bind (_roll _pitch _yaw) (Math|Rotator|BreakRotator _originalrotation))
  ;[1 1 1] Open
  (Variables|Default|SetDoorTick 0)
  (if (< (Variables|Default|GetDoorTick) 131) :!label _label
    (Transformation|AddActorLocalRotation "0,1.000000, 0" false false)
    (Math|Integer|IncrementInt (Variables|Default|GetDoorTick)
      (:%20%20
        (Utilities|FlowControl|Delay 0.001)
        (goto _label)))
    (else
      (Transformation|SetActorRelativeRotation (Math|Rotator|MakeRotator _roll _pitch (+ _yaw 1.3e+02)))
      (Variables|Default|SetIsOpen true)
      (Variables|Default|SetIsOpenning false))))

(event EventBeginPlay
  (Variables|Default|SetOriginalRotation (Transformation|GetActorRotation))
  (bind _asnav_link_proxy (Utilities|Casting|CastToNavLinkProxy (Variables|/Script/Engine.ChildActorComponent|GetChildActor (Variables|Default|GetChildActor))))
  (EventDispatchers|BindEventtoOnSmartLinkReached _asnav_link_proxy (delegate Custom|Link%20Reachedd)))

(event Collision|EventActorBeginOverlap
  (params (OtherActor :type Actor%20Object%20Reference)))

(event EventTick
  (params (DeltaSeconds :type Float%20%28single-precision%29)))

(event EventInteract
  (params (Actor :type String))
  ;[1 1 1] Which action to do
  (if (not (Variables|Default|GetIsOpenning))
    (if (Variables|Default|GetIsOpen)
      (CallFunction|CloseDoor)
      (else
        (CallFunction|OpenDoor)))
    (Variables|Default|SetIsOpenning true)))

(fn ConstructionScript)